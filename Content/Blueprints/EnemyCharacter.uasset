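; Enemy character that deals repeated contact damage to the hero and can itself be damaged and killed.
; Overlapping a HeroCharacter stores it and starts a looping half-second timer that applies Damage through the hero's AffectHealth, until that overlap ends.
; Its own AffectHealth event runs CalculateHealth, prints a debug message and, if IsDead, destroys the actor after a short delay.
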(event Custom|DamageTheHero
  ;[1 1 1] Attacking
  (Default|AffectHealth (Variables|Default|GetHero) (Variables|Default|GetDamage)))

(event EventBeginPlay
  (|CallParentFunction) ; This node is disabled and will not be called.\nDrag off pins to build functionality.
)

(event Collision|EventActorBeginOverlap
  (params (OtherActor :type Actor%20Object%20Reference))
  ;[1 1 1] Attacking
  (bind _ashero_character (Utilities|Casting|CastToHeroCharacter OtherActor))
  (Variables|Default|SetHero _ashero_character)
  (Utilities|Time|SetTimerbyFunctionName 0 "DamageTheHero" 0.5 true))

(event EventTick
  (params (DeltaSeconds :type Float%20%28single-precision%29))
  (|CallParentFunction DeltaSeconds) ; This node is disabled and will not be called.\nDrag off pins to build functionality.
)

(event EventAffectHealth
  (params (Delta :type Float%20%28single-precision%29))
  ;[1 1 1] Getting Damaged
  (CallFunction|CalculateHealth Delta)
  (Development|PrintString "oof" true true "(R=0.483333,G=0.014097,B=0.035469,A=1.000000)")
  (if (Variables|Default|GetisDead)
    (Utilities|FlowControl|Delay 0.5)
    (Actor|DestroyActor)))

(event Collision|EventActorEndOverlap
  (params (OtherActor :type Actor%20Object%20Reference))
  ;[1 1 1] Attacking
  (if (== OtherActor (Variables|Default|GetHero))
    (Utilities|Time|ClearTimerbyFunctionName 0 "DamageTheHero")))

(fn ConstructionScript
  (|CallParentFunction))