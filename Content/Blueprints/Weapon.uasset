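; Weapon Blueprint that fires projectiles automatically while its trigger is held.
; PullTrigger, guarded by a DoOnce, fires immediately and starts a looping timer on Fire at an interval derived from RoundsPerSec.
; ReleaseTrigger clears the timer and resets the DoOnce.
; Each Fire spawns the configured Projectile class at the ProjectileSpawnPoint transform.
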(event Custom|PullTrigger
  ;[1 1 1] Pull and Release Trigger
  (Utilities|FlowControl|DoOnce false
    (:Completed
      (CallFunction|Fire)
      (Utilities|Time|SetTimerbyFunctionName 0 "Fire" (/ 1.0 (Variables|Default|GetRoundsPerSec)) true))))

(event Custom|Fire
  ;[1 1 1] Fire
  (Game|SpawnActorfromClass "/Game/Blueprints/Projectile.Projectile_C" (Transformation|GetWorldTransform (Variables|Default|GetProjectileSpawnPoint)) "Undefined" 0 0))

(event Custom|ReleaseTrigger
  ;[1 1 1] Pull and Release Trigger
  (Utilities|Time|ClearTimerbyFunctionName 0 "Fire")
  (Utilities|FlowControl|DoOnce false) ; enters at Reset
)

(event EventBeginPlay)

(event Collision|EventActorBeginOverlap
  (params (OtherActor :type Actor%20Object%20Reference)))

(event EventTick
  (params (DeltaSeconds :type Float%20%28single-precision%29)))

(fn ConstructionScript)